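; BP_Grenade is a grenade actor that damages walking and flying aliens on impact.
; Its first hit against anything other than the player plays an explosion sound, makes noise attributed to the player, and immediately damages aliens overlapping ExplosionRange.
; Damage dispatch uses chained casts to BP_WalkingAlien, then BP_FlyingAlien, with debug prints.
; The particle system spawns only after a delay following damage, then the actor destroys itself.
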(event Custom|DamageObjectsInside
  (for _array_element (Collision|GetOverlappingActors (Variables|Default|GetExplosionRange) 0 :!class /Script/Engine.PrimitiveComponent)
    (bind _asbp_walking_alien (Utilities|Casting|CastToBP_WalkingAlien _array_element)
      (:then
        (Default|TakeDamage _asbp_walking_alien (Variables|Default|GetDamage))
        (Development|PrintString "Walking Alien Explose"))
      (:CastFailed
        (bind _asbp_flying_alien (Utilities|Casting|CastToBP_FlyingAlien _array_element))
        (Default|TakeDamage _asbp_flying_alien (Variables|Default|GetDamage))
        (Development|PrintString "Flying Alien Explose")))))

(event Collision|EventHit
  (params (MyComp :type Primitive%20Component%20Object%20Reference) (Other :type Actor%20Object%20Reference) (OtherComp :type Primitive%20Component%20Object%20Reference) (bSelfMoved :type Boolean) (HitLocation :type Vector :default "0, 0, 0") (HitNormal :type Vector :default "0, 0, 0") (NormalImpulse :type Vector :default "0, 0, 0") (Hit :type Hit%20Result%20Structure%20%28by%20ref%29))
  (bind _returnvalue (Game|GetPlayerCharacter 0))
  (bind _returnvalue_2 (Transformation|GetActorLocation))
  (if (!= Other _returnvalue)
    (Utilities|FlowControl|DoOnce false
      (:Completed
        (Audio|PlaySoundatLocation "/Game/StarterContent/Audio/Explosion02.Explosion02" _returnvalue_2 "0, 0, 0" 1.0 1.0 0.0 0 0 0 0)
        (Class|Actor|MakeNoise 1.0 _returnvalue _returnvalue_2 0.0 "None")
        (CallFunction|DamageObjectsInside)
        (Utilities|FlowControl|Delay 5.0)
        (Niagara|SpawnSystematLocation 0 (Transformation|GetActorLocation))
        (Actor|DestroyActor)))))

(fn ConstructionScript)