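; Boss-area force field actor made of six mesh panels, each with its own trigger box, that changes its material as the player approaches.
; BeginPlay gives each panel a dynamic material instance.
; When BP_FirstPersonCharacter enters a box, that panel's timeline lerps a scalar material parameter from 1 to 0.
; Leaving the box reverses the timeline from its end, restoring the value independently per panel.
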(event OnComponentBeginOverlap(Box2)
  (params (OverlappedComponent :type Primitive%20Component%20Object%20Reference) (OtherActor :type Actor%20Object%20Reference) (OtherComp :type Primitive%20Component%20Object%20Reference) (OtherBodyIndex :type Integer) (bFromSweep :type Boolean) (SweepResult :type Hit%20Result%20Structure%20%28by%20ref%29))
  (Utilities|Casting|CastToBP_FirstPersonCharacter OtherActor)
  (bind _timeline_forcefield (Timeline|Timeline_1 Play)
    (:Update
      (Rendering|Material|SetScalarParameterValue (Variables|Default|GetDynamic%20Material%20Reference%205) (Variables|Default|GetParameter%20Name) (Math|Float|Lerp 1.0 0.0 _timeline_forcefield) :!class /Script/Engine.MaterialInstanceDynamic))))

(event OnComponentEndOverlap(Box2)
  (params (OverlappedComponent :type Primitive%20Component%20Object%20Reference) (OtherActor :type Actor%20Object%20Reference) (OtherComp :type Primitive%20Component%20Object%20Reference) (OtherBodyIndex :type Integer))
  (Utilities|Casting|CastToBP_FirstPersonCharacter OtherActor)
  (bind _timeline_forcefield (Timeline|Timeline_1 ReverseFromEnd)
    (:Update
      (Rendering|Material|SetScalarParameterValue (Variables|Default|GetDynamic%20Material%20Reference%205) (Variables|Default|GetParameter%20Name) (Math|Float|Lerp 1.0 0.0 _timeline_forcefield) :!class /Script/Engine.MaterialInstanceDynamic))))

(event OnComponentBeginOverlap(Box3)
  (params (OverlappedComponent :type Primitive%20Component%20Object%20Reference) (OtherActor :type Actor%20Object%20Reference) (OtherComp :type Primitive%20Component%20Object%20Reference) (OtherBodyIndex :type Integer) (bFromSweep :type Boolean) (SweepResult :type Hit%20Result%20Structure%20%28by%20ref%29))
  (Utilities|Casting|CastToBP_FirstPersonCharacter OtherActor)
  (bind _timeline_forcefield (Timeline|Timeline_3 Play)
    (:Update
      (Rendering|Material|SetScalarParameterValue (Variables|Default|GetDynamic%20Material%20Reference%202) (Variables|Default|GetParameter%20Name) (Math|Float|Lerp 1.0 0.0 _timeline_forcefield) :!class /Script/Engine.MaterialInstanceDynamic))))

(event OnComponentBeginOverlap(Box4)
  (params (OverlappedComponent :type Primitive%20Component%20Object%20Reference) (OtherActor :type Actor%20Object%20Reference) (OtherComp :type Primitive%20Component%20Object%20Reference) (OtherBodyIndex :type Integer) (bFromSweep :type Boolean) (SweepResult :type Hit%20Result%20Structure%20%28by%20ref%29))
  (Utilities|Casting|CastToBP_FirstPersonCharacter OtherActor)
  (bind _timeline_forcefield (Timeline|Timeline_2 Play)
    (:Update
      (Rendering|Material|SetScalarParameterValue (Variables|Default|GetDynamic%20Material%20Reference%203) (Variables|Default|GetParameter%20Name) (Math|Float|Lerp 1.0 0.0 _timeline_forcefield) :!class /Script/Engine.MaterialInstanceDynamic))))

(event OnComponentEndOverlap(Box3)
  (params (OverlappedComponent :type Primitive%20Component%20Object%20Reference) (OtherActor :type Actor%20Object%20Reference) (OtherComp :type Primitive%20Component%20Object%20Reference) (OtherBodyIndex :type Integer))
  (Utilities|Casting|CastToBP_FirstPersonCharacter OtherActor)
  (bind _timeline_forcefield (Timeline|Timeline_3 ReverseFromEnd)
    (:Update
      (Rendering|Material|SetScalarParameterValue (Variables|Default|GetDynamic%20Material%20Reference%202) (Variables|Default|GetParameter%20Name) (Math|Float|Lerp 1.0 0.0 _timeline_forcefield) :!class /Script/Engine.MaterialInstanceDynamic))))

(event OnComponentEndOverlap(Box4)
  (params (OverlappedComponent :type Primitive%20Component%20Object%20Reference) (OtherActor :type Actor%20Object%20Reference) (OtherComp :type Primitive%20Component%20Object%20Reference) (OtherBodyIndex :type Integer))
  (Utilities|Casting|CastToBP_FirstPersonCharacter OtherActor)
  (bind _timeline_forcefield (Timeline|Timeline_2 ReverseFromEnd)
    (:Update
      (Rendering|Material|SetScalarParameterValue (Variables|Default|GetDynamic%20Material%20Reference%203) (Variables|Default|GetParameter%20Name) (Math|Float|Lerp 1.0 0.0 _timeline_forcefield) :!class /Script/Engine.MaterialInstanceDynamic))))

(event OnComponentBeginOverlap(Box5)
  (params (OverlappedComponent :type Primitive%20Component%20Object%20Reference) (OtherActor :type Actor%20Object%20Reference) (OtherComp :type Primitive%20Component%20Object%20Reference) (OtherBodyIndex :type Integer) (bFromSweep :type Boolean) (SweepResult :type Hit%20Result%20Structure%20%28by%20ref%29))
  (Utilities|Casting|CastToBP_FirstPersonCharacter OtherActor)
  (bind _timeline_forcefield (Timeline|Timeline_4 Play)
    (:Update
      (Rendering|Material|SetScalarParameterValue (Variables|Default|GetDynamic%20Material%20Reference%204) (Variables|Default|GetParameter%20Name) (Math|Float|Lerp 1.0 0.0 _timeline_forcefield) :!class /Script/Engine.MaterialInstanceDynamic))))

(event OnComponentEndOverlap(Box5)
  (params (OverlappedComponent :type Primitive%20Component%20Object%20Reference) (OtherActor :type Actor%20Object%20Reference) (OtherComp :type Primitive%20Component%20Object%20Reference) (OtherBodyIndex :type Integer))
  (Utilities|Casting|CastToBP_FirstPersonCharacter OtherActor)
  (bind _timeline_forcefield (Timeline|Timeline_4 ReverseFromEnd)
    (:Update
      (Rendering|Material|SetScalarParameterValue (Variables|Default|GetDynamic%20Material%20Reference%204) (Variables|Default|GetParameter%20Name) (Math|Float|Lerp 1.0 0.0 _timeline_forcefield) :!class /Script/Engine.MaterialInstanceDynamic))))

(event OnComponentBeginOverlap(Box1)
  (params (OverlappedComponent :type Primitive%20Component%20Object%20Reference) (OtherActor :type Actor%20Object%20Reference) (OtherComp :type Primitive%20Component%20Object%20Reference) (OtherBodyIndex :type Integer) (bFromSweep :type Boolean) (SweepResult :type Hit%20Result%20Structure%20%28by%20ref%29))
  (Utilities|Casting|CastToBP_FirstPersonCharacter OtherActor)
  (bind _timeline_forcefield (Timeline|Timeline_0 Play)
    (:Update
      (Rendering|Material|SetScalarParameterValue (Variables|Default|GetDynamic%20Material%20Reference%201) (Variables|Default|GetParameter%20Name) (Math|Float|Lerp 1.0 0.0 _timeline_forcefield) :!class /Script/Engine.MaterialInstanceDynamic))))

(event OnComponentEndOverlap(Box1)
  (params (OverlappedComponent :type Primitive%20Component%20Object%20Reference) (OtherActor :type Actor%20Object%20Reference) (OtherComp :type Primitive%20Component%20Object%20Reference) (OtherBodyIndex :type Integer))
  (Utilities|Casting|CastToBP_FirstPersonCharacter OtherActor)
  (bind _timeline_forcefield (Timeline|Timeline_0 ReverseFromEnd)
    (:Update
      (Rendering|Material|SetScalarParameterValue (Variables|Default|GetDynamic%20Material%20Reference%201) (Variables|Default|GetParameter%20Name) (Math|Float|Lerp 1.0 0.0 _timeline_forcefield) :!class /Script/Engine.MaterialInstanceDynamic))))

(event OnComponentBeginOverlap(Box)
  (params (OverlappedComponent :type Primitive%20Component%20Object%20Reference) (OtherActor :type Actor%20Object%20Reference) (OtherComp :type Primitive%20Component%20Object%20Reference) (OtherBodyIndex :type Integer) (bFromSweep :type Boolean) (SweepResult :type Hit%20Result%20Structure%20%28by%20ref%29))
  (Utilities|Casting|CastToBP_FirstPersonCharacter OtherActor)
  (bind _timeline_forcefield (Timeline|Timeline Play)
    (:Update
      (Rendering|Material|SetScalarParameterValue (Variables|Default|GetDynamic%20Material%20Reference%200) (Variables|Default|GetParameter%20Name) (Math|Float|Lerp 1.0 0.0 _timeline_forcefield) :!class /Script/Engine.MaterialInstanceDynamic))))

(event OnComponentEndOverlap(Box)
  (params (OverlappedComponent :type Primitive%20Component%20Object%20Reference) (OtherActor :type Actor%20Object%20Reference) (OtherComp :type Primitive%20Component%20Object%20Reference) (OtherBodyIndex :type Integer))
  (Utilities|Casting|CastToBP_FirstPersonCharacter OtherActor)
  (bind _timeline_forcefield (Timeline|Timeline ReverseFromEnd)
    (:Update
      (Rendering|Material|SetScalarParameterValue (Variables|Default|GetDynamic%20Material%20Reference%200) (Variables|Default|GetParameter%20Name) (Math|Float|Lerp 1.0 0.0 _timeline_forcefield) :!class /Script/Engine.MaterialInstanceDynamic))))

(event EventBeginPlay
  (bind _returnvalue (Rendering|Material|CreateDynamicMaterialInstance (Rendering|Material|GetMaterial (Variables|Default|GetStaticMesh) 0) "None" "None" :!class /Script/Engine.KismetMaterialLibrary))
  (bind _output_get (Variables|Default|SetDynamic%20Material%20Reference%200 _returnvalue))
  (Rendering|Material|SetMaterial (Variables|Default|GetStaticMesh) 0 _output_get)
  (bind _returnvalue_2 (Rendering|Material|CreateDynamicMaterialInstance (Rendering|Material|GetMaterial (Variables|Default|GetStaticMesh1) 0) "None" "None" :!class /Script/Engine.KismetMaterialLibrary))
  (bind _output_get_2 (Variables|Default|SetDynamic%20Material%20Reference%201 _returnvalue_2))
  (Rendering|Material|SetMaterial (Variables|Default|GetStaticMesh1) 0 _output_get_2)
  (bind _returnvalue_3 (Rendering|Material|CreateDynamicMaterialInstance (Rendering|Material|GetMaterial (Variables|Default|GetStaticMesh2) 0) "None" "None" :!class /Script/Engine.KismetMaterialLibrary))
  (bind _output_get_3 (Variables|Default|SetDynamic%20Material%20Reference%202 _returnvalue_3))
  (Rendering|Material|SetMaterial (Variables|Default|GetStaticMesh2) 0 _output_get_3)
  (bind _returnvalue_4 (Rendering|Material|CreateDynamicMaterialInstance (Rendering|Material|GetMaterial (Variables|Default|GetStaticMesh3) 0) "None" "None" :!class /Script/Engine.KismetMaterialLibrary))
  (bind _output_get_4 (Variables|Default|SetDynamic%20Material%20Reference%203 _returnvalue_4))
  (Rendering|Material|SetMaterial (Variables|Default|GetStaticMesh3) 0 _output_get_4)
  (bind _returnvalue_5 (Rendering|Material|CreateDynamicMaterialInstance (Rendering|Material|GetMaterial (Variables|Default|GetStaticMesh4) 0) "None" "None" :!class /Script/Engine.KismetMaterialLibrary))
  (bind _output_get_5 (Variables|Default|SetDynamic%20Material%20Reference%204 _returnvalue_5))
  (Rendering|Material|SetMaterial (Variables|Default|GetStaticMesh4) 0 _output_get_5)
  (bind _returnvalue_6 (Rendering|Material|CreateDynamicMaterialInstance (Rendering|Material|GetMaterial (Variables|Default|GetStaticMesh5) 0) "None" "None" :!class /Script/Engine.KismetMaterialLibrary))
  (bind _output_get_6 (Variables|Default|SetDynamic%20Material%20Reference%205 _returnvalue_6))
  (Rendering|Material|SetMaterial (Variables|Default|GetStaticMesh5) 0 _output_get_6))

(fn ConstructionScript)