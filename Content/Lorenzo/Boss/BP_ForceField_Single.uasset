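; BP_ForceField_Single is a force field actor that visually reacts when the first-person character enters or leaves its trigger box.
; On BeginPlay it creates a dynamic material instance for its static mesh.
; Overlap shows a point light and plays a timeline that lerps a material scalar parameter from 1 toward 0.
; Ending the overlap hides the light and reverses the timeline.
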(event OnComponentBeginOverlap(Box1)
  (params (OverlappedComponent :type Primitive%20Component%20Object%20Reference) (OtherActor :type Actor%20Object%20Reference) (OtherComp :type Primitive%20Component%20Object%20Reference) (OtherBodyIndex :type Integer) (bFromSweep :type Boolean) (SweepResult :type Hit%20Result%20Structure%20%28by%20ref%29))
  (Utilities|Casting|CastToBP_FirstPersonCharacter OtherActor)
  (Rendering|SetVisibility (Variables|Default|GetPointLight) true false)
  (bind _timeline_forcefield (Timeline|Timeline_0 Play)
    (:Update
      (Rendering|Material|SetScalarParameterValue (Variables|Default|GetDynamic%20Material%20Reference%201) (Variables|Default|GetParameter%20Name) (Math|Float|Lerp 1.0 0.0 _timeline_forcefield) :!class /Script/Engine.MaterialInstanceDynamic))))

(event OnComponentEndOverlap(Box1)
  (params (OverlappedComponent :type Primitive%20Component%20Object%20Reference) (OtherActor :type Actor%20Object%20Reference) (OtherComp :type Primitive%20Component%20Object%20Reference) (OtherBodyIndex :type Integer))
  (Utilities|Casting|CastToBP_FirstPersonCharacter OtherActor)
  (Rendering|SetVisibility (Variables|Default|GetPointLight) false false)
  (bind _timeline_forcefield (Timeline|Timeline_0 Reverse)
    (:Update
      (Rendering|Material|SetScalarParameterValue (Variables|Default|GetDynamic%20Material%20Reference%201) (Variables|Default|GetParameter%20Name) (Math|Float|Lerp 1.0 0.0 _timeline_forcefield) :!class /Script/Engine.MaterialInstanceDynamic))))

(event EventBeginPlay
  (bind _returnvalue (Rendering|Material|CreateDynamicMaterialInstance (Rendering|Material|GetMaterial (Variables|Default|GetStaticMesh1) 0) "None" "None" :!class /Script/Engine.KismetMaterialLibrary))
  (bind _output_get (Variables|Default|SetDynamic%20Material%20Reference%201 _returnvalue))
  (Rendering|Material|SetMaterial (Variables|Default|GetStaticMesh1) 0 _output_get))

(fn ConstructionScript)