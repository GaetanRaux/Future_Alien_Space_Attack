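; BP_GrenadesSpawner is a spawner actor that periodically spawns an actor, presumably a grenade, at its root component's location.
; Only a spawner with CanSpawn set starts on BeginPlay, after a fixed delay.
; Each SpawnGrenade call spawns, waits the same delay, then calls SpawnGrenade on OtherSpawner, passing the turn along so linked spawners can alternate in a timed relay.
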(event Custom|SpawnGrenade
  (Game|SpawnActorfromClass "/Game/FirstPerson/Blueprints/BP_Pickup_Grenade.BP_Pickup_Grenade_C" (Math|Transform|MakeTransform (Transformation|GetWorldLocation (Variables|Default|GetDefaultSceneRoot)) "0, 0, 0" "1.000000,1.000000,1.000000") "Undefined" "MultiplyWithRoot" 0 0)
  (Utilities|FlowControl|Delay 15.0)
  (CallFunction|SpawnGrenade (Variables|Default|GetOtherSpawner)))

(event EventBeginPlay
  (if (Variables|Default|GetCanSpawn)
    (Utilities|FlowControl|Delay 15.0)
    (CallFunction|SpawnGrenade)))

(fn ConstructionScript)