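; Player character for a first-person-style horror game with a monster, handling movement, crouch, run, pause, level timer and ambience.
; Tick makes noise scaled to the character's max speed while moving, and MonsterTouch plays death effects before opening the death menu.
; Interact line-traces from the camera to open doors and fridges and counts keys from overlapping interface actors.
; Throwing launches a physics rock, briefly freezing movement during a montage, as interacting does.
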(event Custom|CustomEvent
  (Variables|Default|Setclicked false)
  (Variables|/Script/Engine.CharacterMovementComponent|SetMaxWalkSpeed (Variables|Character|GetCharacterMovement) 1.5e+02)
  (Animation|StopAnimMontage "/Game/Animations/Player/MCO_Mocap/AM_PickUp.AM_PickUp"))

(event Custom|Monster%20Touch
  (Development|PrintString "I'm touched!")
  (bind _returnvalue (UserInterface|CreateWidget "/Game/Blueprints/Widgets/WBP_Blackscreen.WBP_Blackscreen_C"))
  (UserInterface|Viewport|AddtoViewport _returnvalue 0)
  (Audio|PlaySound2D "/Game/Sounds/Player/Death/SC_Death.SC_Death" 1.0 1.0 0.0 0 0)
  (Audio|PlaySound2D "/Game/Sounds/Monster/MONSTER_SCREAM_______.MONSTER_SCREAM_______" 1.0 1.0 0.0 0 0)
  (Utilities|FlowControl|Delay 4.0)
  (Game|OpenLevel(byObjectReference) "/Game/Levels/L_DeathMenu.L_DeathMenu"))

(event Custom|StopAnimPickUP
  ;[1 1 1] Player interaction and door openning
  (Variables|Default|Setclicked false)
  (Variables|/Script/Engine.CharacterMovementComponent|SetMaxWalkSpeed (Variables|Character|GetCharacterMovement) 1.5e+02)
  (Animation|StopAnimMontage "/Game/Animations/Player/MCO_Mocap/AM_PickUp.AM_PickUp"))

(event Custom|setTimerPause
  (bind _timerreference (Variables|Default|GettimerReference))
  (Utilities|IsValid _timerreference
    (:Is%20Valid
      (if (Game|IsGamePaused)
        (Variables|/Game/Blueprints/Widgets/WBP_Timer.WBP_Timer_C|SetisPaused _timerreference true)
        (else
          (Variables|/Game/Blueprints/Widgets/WBP_Timer.WBP_Timer_C|SetisPaused _timerreference false))))))

(event Input|EnhancedActionEvents|EnhancedInputActionIA_MyCrouch
  (params (ActionValue :type Boolean) (ElapsedSeconds :type Float%20%28double-precision%29) (TriggeredSeconds :type Float%20%28double-precision%29) (InputAction :type Input%20Action%20Object%20Reference :default "/Game/Inputs/Actions/IA_MyCrouch.IA_MyCrouch"))
  ;[1 1 1] Player crouching
  (:Started
    (Character|Crouch))
  (:Completed
    (Character|UnCrouch)))

(event Input|EnhancedActionEvents|EnhancedInputActionIA_MyLook
  (params (ActionValue :type Vector%202D%20Structure) (ElapsedSeconds :type Float%20%28double-precision%29) (TriggeredSeconds :type Float%20%28double-precision%29) (InputAction :type Input%20Action%20Object%20Reference :default "/Game/Inputs/Actions/IA_MyLook.IA_MyLook"))
  ;[1 1 1] Player looking
  (Pawn|Input|AddControllerYawInput (.x ActionValue))
  (Pawn|Input|AddControllerPitchInput (.y ActionValue)))

(event Input|EnhancedActionEvents|EnhancedInputActionIA_Myinteraction
  (params (ActionValue :type Boolean) (ElapsedSeconds :type Float%20%28double-precision%29) (TriggeredSeconds :type Float%20%28double-precision%29) (InputAction :type Input%20Action%20Object%20Reference :default "/Game/Inputs/Actions/IA_Myinteraction.IA_Myinteraction"))
  (bind _playercam (Variables|Default|GetPlayerCam))
  (bind _returnvalue (Transformation|GetWorldLocation _playercam))
  ;[1 1 1] Player fridge openning
  (bind (_outhit _returnvalue_2) (Collision|LineTraceByChannel _returnvalue (+ _returnvalue (* (Math|Vector|GetForwardVector _playercam) 1.5e+02)) "TraceTypeQuery1" false 0 "ForDuration" true "(R=1.000000,G=0.000000,B=0.000000,A=1.000000)" "(R=0.000000,G=1.000000,B=0.000000,A=1.000000)" 1.0))
  (Utilities|FlowControl|Delay 0.2)
  (if _returnvalue_2
    (bind _asbp_fridge (Utilities|Casting|CastToBP_Fridge (.HitActor (Collision|BreakHitResult _outhit))))
    (Default|OpenFridge _asbp_fridge)))

(event Input|EnhancedActionEvents|EnhancedInputActionIA_ShowKeys
  (params (ActionValue :type Boolean) (ElapsedSeconds :type Float%20%28double-precision%29) (TriggeredSeconds :type Float%20%28double-precision%29) (InputAction :type Input%20Action%20Object%20Reference :default "/Game/Inputs/Actions/IA_ShowKeys.IA_ShowKeys"))
  (bind _returnvalue (UserInterface|CreateWidget "/Game/Blueprints/Widgets/inGame/WBP_KeyMessage.WBP_KeyMessage_C"))
  (bind _returnvalue_2 (Game|SpawnActorfromClass "/Game/Blueprints/BP_DisplayWidget.BP_DisplayWidget_C" (Transformation|GetActorTransform) "Undefined" "MultiplyWithRoot" 0 0))
  (Default|DisplayWidget _returnvalue_2 (Utilities|Text|ToText(String) (Utilities|String|Append (Utilities|String|ToString(Text) (Variables|Default|Gettext)) (Utilities|String|ToString(Text) (Utilities|Text|ToText(Integer) (Variables|Default|Getnbr_keys))))) _returnvalue 2.0))

(event Input|EnhancedActionEvents|EnhancedInputActionIA_MyMove
  (params (ActionValue :type Vector%202D%20Structure) (ElapsedSeconds :type Float%20%28double-precision%29) (TriggeredSeconds :type Float%20%28double-precision%29) (InputAction :type Input%20Action%20Object%20Reference :default "/Game/Inputs/Actions/IA_MyMove.IA_MyMove"))
  ;[1 1 1] Player Movement
  (Pawn|Input|AddMovementInput (Math|Vector|GetRightVector (Math|Rotator|MakeRotator 0.0 0.0 (.yaw (Pawn|GetControlRotation :!class /Script/Engine.Pawn)))) (.x ActionValue) false)
  (Pawn|Input|AddMovementInput (Math|Vector|GetForwardVector (Math|Rotator|MakeRotator 0.0 0.0 (.yaw (Pawn|GetControlRotation :!class /Script/Engine.Pawn)))) (.y ActionValue) false))

(event Input|EnhancedActionEvents|EnhancedInputActionIA_MyRun
  (params (ActionValue :type Boolean) (ElapsedSeconds :type Float%20%28double-precision%29) (TriggeredSeconds :type Float%20%28double-precision%29) (InputAction :type Input%20Action%20Object%20Reference :default "/Game/Inputs/Actions/IA_MyRun.IA_MyRun"))
  (bind _charactermovement (Variables|Character|GetCharacterMovement))
  ;[1 1 1] Player Running
  (:Started
    (Variables|/Script/Engine.CharacterMovementComponent|SetMaxWalkSpeed _charactermovement 4.5e+02))
  (:Completed
    (Variables|/Script/Engine.CharacterMovementComponent|SetMaxWalkSpeed _charactermovement 1.5e+02)))

(event Input|EnhancedActionEvents|EnhancedInputActionIA_Myinteraction
  (params (ActionValue :type Boolean) (ElapsedSeconds :type Float%20%28double-precision%29) (TriggeredSeconds :type Float%20%28double-precision%29) (InputAction :type Input%20Action%20Object%20Reference :default "/Game/Inputs/Actions/IA_Myinteraction.IA_Myinteraction"))
  (bind _playercam (Variables|Default|GetPlayerCam))
  (bind _returnvalue (Transformation|GetWorldLocation _playercam))
  ;[1 1 1] Player interaction and door openning
  (:Started
    (Variables|Default|Setclicked true)
    (Variables|/Script/Engine.CharacterMovementComponent|SetMaxWalkSpeed (Variables|Character|GetCharacterMovement) 0.0)
    (Animation|PlayAnimMontage "/Game/Animations/Player/MCO_Mocap/AM_PickUp.AM_PickUp" 1.0 "None")
    (Utilities|Time|SetTimerbyEvent (delegate Custom|StopAnimPickUP) 1.5)
    (bind (_outhit _returnvalue_2) (Collision|LineTraceByChannel _returnvalue (+ _returnvalue (* (Math|Vector|GetForwardVector _playercam) 175.0)) "TraceTypeQuery1" false 0 "ForDuration" true "(R=1.000000,G=0.000000,B=0.000000,A=1.000000)" "(R=0.000000,G=1.000000,B=0.000000,A=1.000000)" 1.0))
    (if _returnvalue_2
      (if (Actor|ActorHasTag (.HitActor (Collision|BreakHitResult _outhit)) "Door")
        (bind _asbp_door (Utilities|Casting|CastToBP_Door (.HitActor (Collision|BreakHitResult _outhit))))
        (Default|OpenDoor _asbp_door)))))

(event Input|EnhancedActionEvents|EnhancedInputActionIA_Pause
  (params (ActionValue :type Boolean) (ElapsedSeconds :type Float%20%28double-precision%29) (TriggeredSeconds :type Float%20%28double-precision%29) (InputAction :type Input%20Action%20Object%20Reference :default "/Game/Inputs/Actions/IA_Pause.IA_Pause"))
  (bind _returnvalue (Game|GetPlayerController 0))
  ;[1 1 1] Game in pause
  (:Started
    (bind _returnvalue_2 (UserInterface|CreateWidget "/Game/Blueprints/Widgets/WBP_PauseMenu.WBP_PauseMenu_C"))
    (UserInterface|Viewport|AddtoViewport _returnvalue_2 0)
    (Variables|/Script/Engine.PlayerController|SetbShowMouseCursor _returnvalue true)
    (Input|SetInputModeUIOnly _returnvalue 0 "DoNotLock" false)
    (Game|SetGamePaused true)))

(event Input|EnhancedActionEvents|EnhancedInputActionIA_Myinteraction
  (params (ActionValue :type Boolean) (ElapsedSeconds :type Float%20%28double-precision%29) (TriggeredSeconds :type Float%20%28double-precision%29) (InputAction :type Input%20Action%20Object%20Reference :default "/Game/Inputs/Actions/IA_Myinteraction.IA_Myinteraction"))
  ;[1 1 1] Player key interaction
  (for _array_element (Collision|GetOverlappingActors 0 :!class /Script/Engine.Actor)
    (if (Utilities|DoesObjectImplementInterface _array_element "/Game/Blueprints/Coins/BPI_Interact.BPI_Interact_C")
      (Class|BPIInteract|NewFunction(Message) _array_element)
      (bind _output_get (Variables|Default|Setnbr_keys (+ (Variables|Default|Getnbr_keys) 1)))
      (Development|PrintString (Utilities|String|ToString(Integer) _output_get)))))

(event Input|EnhancedActionEvents|EnhancedInputActionIA_Myinteraction
  (params (ActionValue :type Boolean) (ElapsedSeconds :type Float%20%28double-precision%29) (TriggeredSeconds :type Float%20%28double-precision%29) (InputAction :type Input%20Action%20Object%20Reference :default "/Game/Inputs/Actions/IA_Myinteraction.IA_Myinteraction"))
  (bind _playercam (Variables|Default|GetPlayerCam))
  (bind _returnvalue (Transformation|GetWorldLocation _playercam))
  ;[1 1 1] Player open indoor
  (bind (_outhit _returnvalue_2) (Collision|LineTraceByChannel _returnvalue (+ _returnvalue (* (Math|Vector|GetForwardVector _playercam) 1.5e+02)) "TraceTypeQuery1" false 0 "ForDuration" true "(R=1.000000,G=0.000000,B=0.000000,A=1.000000)" "(R=0.000000,G=1.000000,B=0.000000,A=1.000000)" 1.0))
  (Utilities|FlowControl|Delay 0.2)
  (if _returnvalue_2
    (bind _asbp_in_door (Utilities|Casting|CastToBP_InDoor (.HitActor (Collision|BreakHitResult _outhit))))
    (Default|OpeninDoor _asbp_in_door)))

(event Input|EnhancedActionEvents|EnhancedInputActionIA_Throw
  (params (ActionValue :type Boolean) (ElapsedSeconds :type Float%20%28double-precision%29) (TriggeredSeconds :type Float%20%28double-precision%29) (InputAction :type Input%20Action%20Object%20Reference :default "/Game/Inputs/Actions/IA_Throw.IA_Throw"))
  (Variables|Default|Setclicked true)
  (Variables|/Script/Engine.CharacterMovementComponent|SetMaxWalkSpeed (Variables|Character|GetCharacterMovement) 0.0)
  (Animation|PlayAnimMontage "/Game/Animations/Player/MCO_Mocap/AM_PickUp.AM_PickUp" 25.0 "None")
  (Utilities|Time|SetTimerbyEvent (delegate Custom|CustomEvent) 1.5)
  (bind _returnvalue (Game|SpawnActorfromClass "/Game/Blueprints/BP_Rock.BP_Rock_C" (Math|Transform|MakeTransform (Transformation|GetWorldLocation (Variables|Default|GetRockSpawnLocation)) (Transformation|GetActorRotation) "1.000000,1.000000,1.000000") "Undefined" "MultiplyWithRoot" 0 0))
  (Physics|SetPhysicsLinearVelocity (Variables|/Game/Blueprints/BP_Rock.BP_Rock_C|GetSphere1 _returnvalue) (* (Math|Vector|GetUnitDirection(Vector) (Transformation|GetActorLocation) (Transformation|GetActorLocation _returnvalue)) "1000.000000,1000.000000,1000.000000") false "None"))

(event Input|EnhancedActionEvents|EnhancedInputActionIA_Myinteraction
  (params (ActionValue :type Boolean) (ElapsedSeconds :type Float%20%28double-precision%29) (TriggeredSeconds :type Float%20%28double-precision%29) (InputAction :type Input%20Action%20Object%20Reference :default "/Game/Inputs/Actions/IA_Myinteraction.IA_Myinteraction"))
  (bind _playercam (Variables|Default|GetPlayerCam))
  (bind _returnvalue (Transformation|GetWorldLocation _playercam))
  ;[1 1 1] Player double door openning
  (bind (_outhit _returnvalue_2) (Collision|LineTraceByChannel _returnvalue (+ _returnvalue (* (Math|Vector|GetForwardVector _playercam) 1.5e+02)) "TraceTypeQuery1" false 0 "ForDuration" true "(R=1.000000,G=0.000000,B=0.000000,A=1.000000)" "(R=0.000000,G=1.000000,B=0.000000,A=1.000000)" 1.0))
  (Utilities|FlowControl|Delay 0.2)
  (if _returnvalue_2
    (bind _asbp_double_door (Utilities|Casting|CastToBP_DoubleDoor (.HitActor (Collision|BreakHitResult _outhit)))
      (:then
        (Default|OpenDoubleDoor _asbp_double_door))
      (:CastFailed
        (Development|PrintString "double door openning failed")))))

(event EventBeginPlay
  (bind _returnvalue (Game|GetPlayerController 0))
  (bind _returnvalue_2 (PlayerController|LocalPlayerSubsystems|GetEnhancedInputLocalPlayerSubsystem _returnvalue))
  (bind _returnvalue_3 (Class|EnhancedInputSubsystemInterface|GetUserSettings _returnvalue_2))
  ;[1 1 1] Player Gameplay
  (bind _returnvalue_4 (Game|GetCurrentLevelName true))
  (if (Utilities|Enum|Equal(Enum) _returnvalue_4 "L_MainMenuMansion")
    _
    (else
      (if (Utilities|Enum|Equal(Enum) _returnvalue_4 "L_Tutorial")
        _
        (else
          (bind _returnvalue_5 (UserInterface|CreateWidget "/Game/Blueprints/Widgets/WBP_Timer.WBP_Timer_C"))
          (bind _output_get (Variables|Default|SettimerReference _returnvalue_5))
          (UserInterface|Viewport|AddtoViewport _returnvalue_5 0)))
      (Audio|SpawnSound2D "/Game/Sounds/Ambiance/Horror_ambiance_sound.Horror_ambiance_sound" 1.0 1.0 0.0 0)))
  (Utilities|IsValid _returnvalue_2
    (:Is%20Valid
      (Input|AddMappingContext _returnvalue_2 "/Game/Inputs/IMC_Player.IMC_Player" 0 "(bIgnoreAllPressedKeysUntilRelease=True,bForceImmediately=False,bNotifyUserSettings=False)")
      (if (Class|EnhancedInputUserSettings|IsMappingContextRegistered _returnvalue_3)
        (Input|SetInputModeGameOnly (Game|GetPlayerController 0) false)
        (else
          (Class|EnhancedInputUserSettings|RegisterInputMappingContext _returnvalue_3 "/Game/Inputs/IMC_Player.IMC_Player")
          (Input|SetInputModeGameOnly (Game|GetPlayerController 0) false))))))

(event EventTick
  (params (DeltaSeconds :type Float%20%28single-precision%29))
  (bind _charactermovement (Variables|Character|GetCharacterMovement))
  (bind _returnvalue (Class|MovementComponent|GetMaxSpeed _charactermovement))
  ;[1 1 1] Player noise maker
  (CallFunction|SetTimerPause)
  (if (!= (Math|Vector|VectorLength (Transformation|GetVelocity)) 0.0)
    (if (== _returnvalue 1e+02)
      (Class|Actor|MakeNoise 0.1 self (Transformation|GetActorLocation) 0.0 "None")
      (elif (== _returnvalue 1.5e+02)
        (Class|Actor|MakeNoise 0.3 self (Transformation|GetActorLocation) 0.0 "None")
        (elif (== _returnvalue 4.5e+02)
          (Class|Actor|MakeNoise 0.5 self (Transformation|GetActorLocation) 0.0 "None"))))))

(event Input|KeyboardEvents|G
  (params (Key :type Key%20Structure :default "None"))
  (:Pressed
    (Class|Actor|MakeNoise 1.0 self (Transformation|GetActorLocation) 0.0 "None")
    (Development|PrintString "Noise")))

(fn ConstructionScript)