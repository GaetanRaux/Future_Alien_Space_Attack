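; BP_Tentacula is a tentacled enemy that provides attack moves for its right arm, a BP_Tentacle child actor.
; Each move sets the tentacle's target location and interpolation speed: hover over player or right target point, crush down, sweep to left target point, or reset to origin.
; Moves print debug text and return a float, apparently a duration, though Sweep returns its interpolation speed.
; Attack is a stub, and no sequencing appears here.
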(fn ConstructionScript)

(fn Attack
  (return 0.0))

(fn TentacleCrush
  (bind _childarmright (Variables|Default|GetChildArmRight))
  (Development|PrintString "Tentacle Crush")
  (Utilities|IsValid _childarmright
    (:Is%20Valid
      (bind _asbp_tentacle (Utilities|Casting|CastToBP_Tentacle (Variables|/Script/Engine.ChildActorComponent|GetChildActor _childarmright)))
      (Variables|/Game/Enemy/BP_Tentacle.BP_Tentacle_C|SetTargetLocation _asbp_tentacle (Math|Vector|MakeVector (.x (Variables|/Game/Enemy/BP_Tentacle.BP_Tentacle_C|GetCurrentLocation _asbp_tentacle)) (.y (Variables|/Game/Enemy/BP_Tentacle.BP_Tentacle_C|GetCurrentLocation _asbp_tentacle)) (- (.z (Variables|/Game/Enemy/BP_Tentacle.BP_Tentacle_C|GetCurrentLocation _asbp_tentacle)) 3.5e+02)))
      (Variables|/Game/Enemy/BP_Tentacle.BP_Tentacle_C|SetInterpolationSpeed _asbp_tentacle 2e+01)
      (return 2.0))))

(fn TentacleOverPlayer
  (bind _returnvalue (Game|GetPlayerCharacter 0))
  (bind _childarmright (Variables|Default|GetChildArmRight))
  (bind _returnvalue_2 (Transformation|GetActorLocation _returnvalue))
  (Development|PrintString "Tentacle Over")
  (Utilities|IsValid _childarmright
    (:Is%20Valid
      (bind _asbp_tentacle (Utilities|Casting|CastToBP_Tentacle (Variables|/Script/Engine.ChildActorComponent|GetChildActor _childarmright)))
      (Variables|/Game/Enemy/BP_Tentacle.BP_Tentacle_C|SetTargetLocation _asbp_tentacle (Math|Vector|MakeVector (.x _returnvalue_2) (.y _returnvalue_2) (+ (.z _returnvalue_2) 3e+02)))
      (Variables|/Game/Enemy/BP_Tentacle.BP_Tentacle_C|SetInterpolationSpeed _asbp_tentacle 5.0)
      (return 2.0))))

(fn TentacleOverTarget
  (bind _childarmright (Variables|Default|GetChildArmRight))
  (bind _righttargetpoint (Variables|Default|GetRightTargetPoint))
  (bind _returnvalue (Transformation|GetActorLocation _righttargetpoint))
  (Development|PrintString "Tentacle Over")
  (Utilities|IsValid _childarmright
    (:Is%20Valid
      (bind _asbp_tentacle (Utilities|Casting|CastToBP_Tentacle (Variables|/Script/Engine.ChildActorComponent|GetChildActor _childarmright)))
      (Variables|/Game/Enemy/BP_Tentacle.BP_Tentacle_C|SetTargetLocation _asbp_tentacle (Math|Vector|MakeVector (.x _returnvalue) (.y _returnvalue) (+ (.z _returnvalue) 4.5e+02)))
      (Variables|/Game/Enemy/BP_Tentacle.BP_Tentacle_C|SetInterpolationSpeed _asbp_tentacle 5.0)
      (return 2.0))))

(fn TentacleReset
  (bind _childarmright (Variables|Default|GetChildArmRight))
  (Development|PrintString "Tentacle Reset")
  (Utilities|IsValid _childarmright
    (:Is%20Valid
      (bind _asbp_tentacle (Utilities|Casting|CastToBP_Tentacle (Variables|/Script/Engine.ChildActorComponent|GetChildActor _childarmright)))
      (Variables|/Game/Enemy/BP_Tentacle.BP_Tentacle_C|SetTargetLocation _asbp_tentacle (Variables|/Game/Enemy/BP_Tentacle.BP_Tentacle_C|GetOriginLocation _asbp_tentacle))
      (Variables|/Game/Enemy/BP_Tentacle.BP_Tentacle_C|SetInterpolationSpeed _asbp_tentacle 2.0)
      (return 5.0))))

(fn TentacleSweep
  (bind _childarmright (Variables|Default|GetChildArmRight))
  (bind _lefttargetpoint (Variables|Default|GetLeftTargetPoint))
  (bind _returnvalue (Transformation|GetActorLocation _lefttargetpoint))
  (Development|PrintString "Tentacle Sweep")
  (Utilities|IsValid _childarmright
    (:Is%20Valid
      (bind _asbp_tentacle (Utilities|Casting|CastToBP_Tentacle (Variables|/Script/Engine.ChildActorComponent|GetChildActor _childarmright)))
      (Variables|/Game/Enemy/BP_Tentacle.BP_Tentacle_C|SetTargetLocation _asbp_tentacle (Math|Vector|MakeVector (.x _returnvalue) (.y _returnvalue) (+ (.z _returnvalue) 1e+02)))
      (bind _output_get (Variables|/Game/Enemy/BP_Tentacle.BP_Tentacle_C|SetInterpolationSpeed _asbp_tentacle 3.0))
      (return _output_get))))