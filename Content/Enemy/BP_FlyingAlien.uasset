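; Flying alien enemy that, once PawnSensing spots the player, sets a blackboard flag, snaps to face them and fires a projectile every second.
; TakeDamage deaths award player XP and ragdoll the mesh briefly before destruction.
; Player projectile overlaps subtract fixed health separately and destroy it on death without XP or ragdoll.
; Attack and tentacle functions are stubs returning constants.
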(event OnSeePawn(PawnSensing)
  (params (Pawn :type Pawn%20Object%20Reference))
  (Utilities|Casting|CastToBP_FirstPersonCharacter Pawn)
  (AI|Components|Blackboard|SetValueasBool (AI|GetBlackboard (AI|GetAIController self)) (Utilities|Name|MakeLiteralName "hasSeenPlayer?") true)
  (Variables|Default|SethasSeenPlayerOneTime? true))

(event Custom|TakeDamage
  (params (AmountOfDamage :type Integer))
  (bind _sk_alien_01 (Variables|Default|GetSK_Alien_01))
  (bind _output_get (Variables|Default|SetHealth (- (Variables|Default|GetHealth) AmountOfDamage)))
  (if (<= _output_get 0)
    (bind _asbp_first_person_character (Utilities|Casting|CastToBP_FirstPersonCharacter (Game|Player|GetPlayerPawn 0))
      (:then
        (Default|AddXP _asbp_first_person_character 5.0)
        (Components|DestroyComponent (Variables|Collision|GetCapsuleComponent))
        (Collision|SetCollisionEnabled _sk_alien_01 "PhysicsOnly")
        (Physics|SetSimulatePhysics _sk_alien_01 true)
        (Utilities|FlowControl|Delay 1.5))
      (:CastFailed
        _))
    (Actor|DestroyActor)))

(event EventTick
  (params (DeltaSeconds :type Float%20%28single-precision%29))
  (if (Variables|Default|GethasSeenPlayerOneTime?)
    (Variables|Default|SetTimeElapsed (+ (Variables|Default|GetTimeElapsed) (Utilities|Time|GetWorldDeltaSeconds)))
    (Transformation|SetActorRotation (Math|Rotator|FindLookatRotation (Transformation|GetActorLocation) (Transformation|GetActorLocation (Game|GetPlayerCharacter 0))))
    (if (>= (Variables|Default|GetTimeElapsed) 1.0)
      (Game|SpawnActorfromClass "/Game/FirstPerson/Blueprints/BP_NewAlienProjectile.BP_NewAlienProjectile_C" (Math|Transform|MakeTransform (Transformation|GetWorldLocation (Variables|Default|GetProjectileSpawnLocation)) (Transformation|GetWorldRotation (Variables|Collision|GetCapsuleComponent))) "Undefined" "OverrideRootScale" 0 0)
      (Variables|Default|SetTimeElapsed 0.0))))

(event Collision|EventActorBeginOverlap
  (params (OtherActor :type Actor%20Object%20Reference))
  (Utilities|Casting|CastToBP_NewProjectile OtherActor)
  (bind _output_get (Variables|Default|SetHealth (- (Variables|Default|GetHealth) 10)))
  (if (<= _output_get 0)
    (Development|PrintString "Flying Enemy Death" true true "(R=1.000000,G=0.028216,B=0.000000,A=1.000000)" 1e+01)
    (Actor|DestroyActor)))

(fn ConstructionScript)

(fn Attack
  (Development|PrintString "Attack")
  (return 5.0))

(fn TentacleCrush
  (params (AnimationDuration_Input :type Float%20%28double-precision%29))
  (return 0.0))

(fn TentacleOverPlayer
  (return 0.0))

(fn TentacleOverTarget
  (return 0.0))

(fn TentacleReset
  (return 0.0))

(fn TentacleSweep
  (return 0.0))