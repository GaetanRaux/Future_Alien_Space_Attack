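; BP_WalkingAlien is an enemy alien pawn that detects the first-person player by sight and sound.
; Its PawnSensing events set the hasSeenPlayer? Blackboard key on its AI controller when they sense BP_FirstPersonCharacter, and nothing here clears it.
; Attack is a placeholder that prints a message and returns a fixed value, while the Tentacle functions are empty stubs returning zero.
; Tick is empty, and a debug print of the seen state is left unconnected.
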(event OnSeePawn(PawnSensing)
  (params (Pawn :type Pawn%20Object%20Reference))
  (Utilities|Casting|CastToBP_FirstPersonCharacter Pawn)
  (AI|Components|Blackboard|SetValueasBool (AI|GetBlackboard (AI|GetAIController self)) (Utilities|Name|MakeLiteralName "hasSeenPlayer?") true))

(event OnHearNoise(PawnSensing)
  (params (Instigator :type Pawn%20Object%20Reference) (Location :type Vector%20%28by%20ref%29 :default "0, 0, 0") (Volume :type Float%20%28single-precision%29))
  (Utilities|Casting|CastToBP_FirstPersonCharacter Instigator)
  (AI|Components|Blackboard|SetValueasBool (AI|GetBlackboard (AI|GetAIController self)) (Utilities|Name|MakeLiteralName "hasSeenPlayer?") true))

(event EventTick
  (params (DeltaSeconds :type Float%20%28single-precision%29)))

(fn ConstructionScript)

(fn Attack
  (Development|PrintString "Walking Attack")
  (return 5.0))

(fn TentacleCrush
  (return 0.0))

(fn TentacleOverPlayer
  (return 0.0))

(fn TentacleOverTarget
  (return 0.0))

(fn TentacleReset
  (return 0.0))

(fn TentacleSweep
  (return 0.0))